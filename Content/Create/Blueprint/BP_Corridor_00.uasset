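; BP_Corridor_00 is a corridor piece whose static mesh is selected in the construction script.
; The script indexes the Souce01 array with Type and assigns the result to SMesh.
; An unconnected chain, which never runs, would add a point light at each mesh socket, sized by LightLength and LightRadius.
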(fn ConstructionScript
  (Components|StaticMesh|SetStaticMesh (Variables|Default|GetSMesh) (Utilities|Array|Get(acopy) (Variables|Default|GetSouce_01) (Variables|Default|GetType))))