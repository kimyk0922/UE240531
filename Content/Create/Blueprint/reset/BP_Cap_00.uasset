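; BP_Cap_00 is a corridor cover that swings open through a UI prompt shown when its trigger box is overlapped.
; Overlap creates WG_Cap_00, plays its CancelHide animation, shows the cursor, disables pawn input and passes itself to the widget.
; Evt_Cap_move, not called within this graph, plays a timeline that pitches the cover open; ending the overlap reverses it.
; Pawn input is not re-enabled here.
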(event OnComponentBeginOverlap(Box)
  (params (OverlappedComponent :type Primitive%20Component%20Object%20Reference) (OtherActor :type Actor%20Object%20Reference) (OtherComp :type Primitive%20Component%20Object%20Reference) (OtherBodyIndex :type Integer) (bFromSweep :type Boolean) (SweepResult :type Hit%20Result%20Structure%20%28by%20ref%29))
  (bind _returnvalue (Game|GetPlayerController 0))
  (bind _returnvalue_2 (UserInterface|CreateWidget "/Game/Create/Blueprint/reset/WG_Cap_00.WG_Cap_00_C" _returnvalue))
  (UserInterface|Viewport|AddtoViewport _returnvalue_2 0)
  (UserInterface|Animation|PlayAnimation _returnvalue_2 (Variables|/Game/Create/Blueprint/reset/WG_Cap_00.WG_Cap_00_C|GetCancel_Hide _returnvalue_2) 0.0 1 "Forward" 1.0 false)
  (bind _returnvalue_3 (Class|MovieSceneSequenceExtensions|GetPlaybackRange (Variables|/Game/Create/Blueprint/reset/WG_Cap_00.WG_Cap_00_C|GetCancel_Hide _returnvalue_2)))
  (Class|SequencerScriptingRangeExtensions|GetEndSeconds _returnvalue_3)
  (Variables|/Script/Engine.PlayerController|SetbShowMouseCursor _returnvalue true)
  (Input|DisableInput (Game|Player|GetPlayerPawn 0) _returnvalue)
  (Variables|/Game/Create/Blueprint/reset/WG_Cap_00.WG_Cap_00_C|SetOpen_int _returnvalue_2 self))

(event OnComponentEndOverlap(Box)
  (params (OverlappedComponent :type Primitive%20Component%20Object%20Reference) (OtherActor :type Actor%20Object%20Reference) (OtherComp :type Primitive%20Component%20Object%20Reference) (OtherBodyIndex :type Integer))
  (bind _newtrack_0 (Timeline|Timeline Reverse)
    (:Update
      (Transformation|SetRelativeRotation (Variables|Default|GetSM_corridor_Cover_01) (Math|Rotator|MakeRotator 0.0 (Math|Float|Lerp 0.0 -1.1e+02 _newtrack_0) 0.0) false false))))

(event Custom|Evt_Cap_move
  (bind _newtrack_0 (Timeline|Timeline Play)
    (:Update
      (Transformation|SetRelativeRotation (Variables|Default|GetSM_corridor_Cover_01) (Math|Rotator|MakeRotator 0.0 (Math|Float|Lerp 0.0 -1.1e+02 _newtrack_0) 0.0) false false))))

(fn ConstructionScript)