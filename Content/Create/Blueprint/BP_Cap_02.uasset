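; BP_Cap_02 is an interactive actor that opens the WG_Cap_02 widget when anything overlaps its Box trigger.
; The overlap shows the mouse cursor, disables player pawn input and hands the widget a self reference.
; Evt_Ani, not called within this Blueprint, plays the SkCap02 skeletal animation once.
; Ending the overlap sets that animation's play rate to zero, and nothing here restores it or the input.
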(event OnComponentBeginOverlap(Box)
  (params (OverlappedComponent :type Primitive%20Component%20Object%20Reference) (OtherActor :type Actor%20Object%20Reference) (OtherComp :type Primitive%20Component%20Object%20Reference) (OtherBodyIndex :type Integer) (bFromSweep :type Boolean) (SweepResult :type Hit%20Result%20Structure%20%28by%20ref%29))
  (bind _returnvalue (Game|GetPlayerController 0))
  (bind _returnvalue_2 (UserInterface|CreateWidget "/Game/Create/Blueprint/WG_Cap_02.WG_Cap_02_C" _returnvalue))
  (UserInterface|Viewport|AddtoViewport _returnvalue_2 0)
  (Variables|/Script/Engine.PlayerController|SetbShowMouseCursor _returnvalue true)
  (Input|DisableInput (Game|Player|GetPlayerPawn 0) _returnvalue)
  (Variables|/Game/Create/Blueprint/WG_Cap_02.WG_Cap_02_C|SetOpen_int_2 _returnvalue_2 self))

(event OnComponentEndOverlap(Box)
  (params (OverlappedComponent :type Primitive%20Component%20Object%20Reference) (OtherActor :type Actor%20Object%20Reference) (OtherComp :type Primitive%20Component%20Object%20Reference) (OtherBodyIndex :type Integer))
  (bind _sk_cap02 (Variables|Default|GetSk_cap02))
  (Components|Timeline|SetPlayRate _sk_cap02 0.0)
  (Audio|Components|Audio|Play _sk_cap02 false))

(event Custom|Evt_Ani
  (bind _sk_cap02 (Variables|Default|GetSk_cap02))
  (Components|Animation|SetAnimation _sk_cap02 "/Game/Create/Mesh/Sk_cap02_Anim.Sk_cap02_Anim")
  (Audio|Components|Audio|Play _sk_cap02 false))

(fn ConstructionScript)