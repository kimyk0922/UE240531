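; BP_Ele is an elevator actor that moves its inside mesh vertically and offers floor selection through a UI widget.
; Either floor trigger's overlap opens WG_Ele, shows the cursor, disables pawn input and hands the widget a self reference.
; Two floor events drive separate FlipFlop timelines that alternately play and reverse.
; Floor 1 lerps between base and raised positions, while Floor 2's lerp endpoints both equal the raised position.
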(event OnComponentBeginOverlap(Florr_1_Triiger)
  (params (OverlappedComponent :type Primitive%20Component%20Object%20Reference) (OtherActor :type Actor%20Object%20Reference) (OtherComp :type Primitive%20Component%20Object%20Reference) (OtherBodyIndex :type Integer) (bFromSweep :type Boolean) (SweepResult :type Hit%20Result%20Structure%20%28by%20ref%29))
  (|Widget_Bridge))

(event OnComponentBeginOverlap(Florr_2_Triiger)
  (params (OverlappedComponent :type Primitive%20Component%20Object%20Reference) (OtherActor :type Actor%20Object%20Reference) (OtherComp :type Primitive%20Component%20Object%20Reference) (OtherBodyIndex :type Integer) (bFromSweep :type Boolean) (SweepResult :type Hit%20Result%20Structure%20%28by%20ref%29))
  (|Widget_Bridge))

(event Custom|Evt_Ele_1
  (|Ele_Move_Set_Floor1))

(event Custom|Evt_Ele_2
  (|Ele_Move_Set_Floor2))

(fn ConstructionScript)