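; BP_Box is an interactive box actor that opens a UI widget on overlap and can spin its cube.
; Any overlap creates WG_Box, shows the mouse cursor, disables player pawn input and gives the widget a reference to the box.
; Evt_Test, not called within this Blueprint, plays a timeline that drives the cube's relative pitch in turns, then resets the timeline's time so it starts over.
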(event OnComponentBeginOverlap(Box)
  (params (OverlappedComponent :type Primitive%20Component%20Object%20Reference) (OtherActor :type Actor%20Object%20Reference) (OtherComp :type Primitive%20Component%20Object%20Reference) (OtherBodyIndex :type Integer) (bFromSweep :type Boolean) (SweepResult :type Hit%20Result%20Structure%20%28by%20ref%29))
  (bind _returnvalue (Game|GetPlayerController 0))
  (bind _returnvalue_2 (UserInterface|CreateWidget "/Game/Create/Blueprint/WG_Box.WG_Box_C" _returnvalue))
  (UserInterface|Viewport|AddtoViewport _returnvalue_2 0)
  (Variables|/Script/Engine.PlayerController|SetbShowMouseCursor _returnvalue true)
  (Input|DisableInput (Game|Player|GetPlayerPawn 0) _returnvalue)
  (Variables|/Game/Create/Blueprint/WG_Box.WG_Box_C|SetBox_Test _returnvalue_2 self))

(event Custom|Evt_Test
  (Utilities|FlowControl|Sequence
    (:then_0
      (bind _rotation (Timeline|Cube_Animation Play)
        (:Update
          (Transformation|SetRelativeRotation (Variables|Default|GetCube) (Math|Rotator|MakeRotator 0.0 (* _rotation 3.6e+02) 0.0) false false))))
    (:then_1
      (Timeline|Cube_Animation SetNewTime))))

(fn ConstructionScript)